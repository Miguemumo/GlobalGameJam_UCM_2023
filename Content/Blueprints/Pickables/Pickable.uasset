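; Pickable actor that bobs in place until the player comes within their PickupRange stat, then homes in on them to be collected.
; Tick switches one-way from idle bobbing between fixed world heights to an accelerating chase that keeps its current Z.
; Once within PickRange, Pick only prints the item's name and destroys the actor.
; The Player reference arrives through Init, and both range checks use full 3D distance.
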(event `Init`
  (params (Player :type "/Game/Blueprints/Player/Player Object Reference"))
  ;[1 1 1] Initializes Player parameter
  (set `self.Player` Player))

(event `self.ReceiveTick`
  (params (DeltaSeconds :type "Float (single-precision)"))
  ;[1 1 1] Tick. If Moving to player, keeps moving. Otherwise, does idle "animation" and checks player range
  (if (`self.MovingToPlayer`)
    (`self.MoveToPlayer` DeltaSeconds)
    (`self.CheckInPickRange`)
    (else
      (`self.IdleMovement` DeltaSeconds)
      (`self.CheckPlayerInRange`))))

(fn `CheckInPickRange`
  (if (<= (`self.GetDistanceToPlayer`) (`self.PickRange`))
    (`self.Pick`)))

(fn `CheckPlayerInRange`
  (bind (_playerstats_weaponspeedincrease _playerstats_weaponsizeincrease _playerstats_weapondurationincrease _playerstats_weaponcooldown _playerstats_maxhealth _playerstats_pickuprange) (break `/Game/Structs/PlayerStats` (`/Game/Blueprints/Player/Player.PlayerStats` (`self.Player`))))
  (if (<= (`self.GetDistanceToPlayer`) _playerstats_pickuprange)
    (set `self.MovingToPlayer` true)))

(fn `GetDistanceToPlayer`
  (returns (Distance :type "Float (double-precision)"))
  (return (`KismetMathLibrary.Vector_Distance` (`self.K2_GetActorLocation` (`self.Player`)) (`self.K2_GetActorLocation`))))

(fn `IdleMovement`
  (params (Delta :type "Float (double-precision)"))
  (locals (OffsetZ :type "Float (double-precision)") (DeltaTime :type "Float (double-precision)"))
  (bind (_returnvalue_x _returnvalue_y _returnvalue_z) (`KismetMathLibrary.BreakVector` (`SceneComponent.K2_GetComponentLocation` (`self.DefaultSceneRoot`))))
  (bind (_returnvalue_x_2 _returnvalue_y_2 _returnvalue_z_2) (`KismetMathLibrary.BreakVector` (`SceneComponent.K2_GetComponentLocation` (`self.DefaultSceneRoot`))))
  (set `local.DeltaTime` Delta)
  (if (`self.GoingUp`)
    (set `local.OffsetZ` (* (`self.IdleSpeed`) (`local.DeltaTime`)))
    (else
      (set `local.OffsetZ` (* (* (`self.IdleSpeed`) -1.0) (`local.DeltaTime`)))))
  (`SceneComponent.K2_AddWorldOffset` (`self.DefaultSceneRoot`) (`KismetMathLibrary.MakeVector` 0.0 0.0 (`local.OffsetZ`)) false false)
  (if (`self.GoingUp`)
    (if (>= _returnvalue_z_2 260.0)
      (set `self.GoingUp` false))
    (elif (<= _returnvalue_z 220.0)
      (set `self.GoingUp` true))))

(fn `MoveToPlayer`
  (params (Delta :type "Float (double-precision)"))
  (locals (DeltaTime :type "Float (double-precision)"))
  (bind (_returnvalue_x _returnvalue_y _returnvalue_z) (`KismetMathLibrary.BreakVector` (`SceneComponent.K2_GetComponentLocation` (`self.DefaultSceneRoot`))))
  (bind (_returnvalue_x_2 _returnvalue_y_2) (`KismetMathLibrary.BreakVector` (`SceneComponent.K2_GetComponentLocation` (`Actor.RootComponent` (`self.Player`)))))
  (bind _output_get (set `local.DeltaTime` Delta))
  (`SceneComponent.K2_AddWorldOffset` (`self.DefaultSceneRoot`) (* _output_get (`KismetMathLibrary.GetDirectionUnitVector` (`KismetMathLibrary.MakeVector` _returnvalue_x _returnvalue_y _returnvalue_z) (`KismetMathLibrary.MakeVector` _returnvalue_x_2 _returnvalue_y_2 _returnvalue_z)) (`self.MoveSpeed`)) false false)
  (set `self.MoveSpeed` (+ (`self.MoveSpeed`) (* (`local.DeltaTime`) (`self.MoveAcceleration`)))))

(fn `Pick`
  (`KismetSystemLibrary.PrintString` (`KismetStringLibrary.Concat_StrStr` "Picked: " (`KismetSystemLibrary.GetDisplayName` self)))
  (`self.K2_DestroyActor`))

(fn `UserConstructionScript`)