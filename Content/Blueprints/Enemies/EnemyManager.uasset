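; Enemy manager that repeatedly spawns the current wave's enemies around the player.
; A looping timer started on BeginPlay reads the active Waves entry and spawns each enemy type in its configured count.
; Spawn positions offset the player's location by random-angle sine and cosine scaled by Radius, ignoring collisions.
; Each enemy is initialized with the wave index and player pawn, and SetWave changes the active wave.
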(event `self.ReceiveBeginPlay`
  (`KismetSystemLibrary.K2_SetTimerDelegate` (delegate `SpawnEnemy`) 5.0 true))

(event `SpawnEnemy`
  (bind _radius (`self.Radius`))
  (bind (_returnvalue_x _returnvalue_y _returnvalue_z) (`KismetMathLibrary.BreakVector` (`self.K2_GetActorLocation` (`GameplayStatics.GetPlayerPawn` 0))))
  (bind (_output_numenemies _output_enemytype) (break `/Game/Blueprints/Enemies/EnemyWave` (`|GetArrayItem` (`self.Waves`) (`self.ActualWave`))))
  (bind _returnvalue (* (`KismetMathLibrary.RandomFloat`) (`KismetMathLibrary.MultiplyByPi` 2.0)))
  (for (_array_element _array_index) _output_numenemies
    (for _ (range _array_element)
      (bind _returnvalue_2 (`|SpawnActorFromClass` (`|GetArrayItem` _output_enemytype _array_index) (`KismetMathLibrary.MakeTransform` (`KismetMathLibrary.MakeVector` (+ _returnvalue_x (* (`KismetMathLibrary.Cos` _returnvalue) _radius)) (+ _returnvalue_y (* (`KismetMathLibrary.Sin` _returnvalue) _radius)) _returnvalue_z)) "AlwaysSpawn" "OverrideRootScale" null null))
      (`/Game/Blueprints/Enemies/BaseEnemy.Init` _returnvalue_2 (`self.ActualWave`) (`GameplayStatics.GetPlayerPawn` 0)))))

(fn `SetWave`
  (params (Wave :type Integer))
  (set `self.ActualWave` Wave))

(fn `UserConstructionScript`)