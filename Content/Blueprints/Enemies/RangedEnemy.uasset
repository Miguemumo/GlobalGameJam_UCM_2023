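; Ranged enemy Blueprint that attacks by firing a projectile at the player.
; It extends the parent's AttackEvent, spawning the configured ProjectileClass at its own transform with a direction toward the player pawn and itself as instigator.
; Each attack also restarts a timeline that drives SquishBillboard's X and Z scale as a squish animation.
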(event `self.Attack_Event`
  (`parent.Attack_Event`)
  (`self.SpawnProjectile`)
  ;[1 0.3901 0.05729] Attack animation
  (bind (_direction _scalex _scalez) (`Timeline|SquishTimeline` :!via `PlayFromStart`)
    (:`Update`
      (`self.SquishBillboard` _scalex _scalez))))

(fn `SpawnProjectile`
  (`|SpawnActorFromClass` (`self.ProjectileClass`) (`self.GetTransform`) "AlwaysSpawn" "OverrideRootScale" null (`KismetMathLibrary.GetDirectionUnitVector` (`self.K2_GetActorLocation` self) (`self.K2_GetActorLocation` (`self.PlayerPawn`))) self))

(fn `UserConstructionScript`
  (`parent.UserConstructionScript`))