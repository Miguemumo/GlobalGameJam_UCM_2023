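; Base enemy that rises from below via a billboard spawn tween, then moves straight toward the player pawn until within a minimum distance.
; Init supplies the wave and player, and Damage reduces health and calls Die at zero.
; Death disables colliders and camera-facing, plays a tipping timeline, then destroys the actor.
; The looping attack timer fires an empty event, and a test delay kills the enemy shortly after spawning.
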(event `Die_Event`
  ;[1 0.1146 0.1146] Die
  (set `self.IsSpawned` false)
  (`ActorComponent.Deactivate` (`self.HitCollider`))
  (`ActorComponent.Deactivate` (`self.HurtCollider`))
  (`/Game/Blueprints/BillboardComponent.SetLookAtCamera` (`self.BillboardComponent`) false)
  (bind (_direction _t) (`Timeline|Timeline` :!via `PlayFromStart`)
    (:`Update`
      (`self.DieTween` _t))
    (:`Finished`
      (`self.K2_DestroyActor`))))

(event `self.ReceiveBeginPlay`
  (add `self.Die` (delegate `Die_Event`))
  (`/Game/Blueprints/BillboardComponent.SetLookAtCamera` (`self.BillboardComponent`) false)
  (bind (_direction _t) (`Timeline|SpawnTimeline` :!via `PlayFromStart`)
    (:`Update`
      (`self.SpawnTween` _t))
    (:`Finished`
      ;[1 1 1] After spawn animation finished
      (set `self.IsSpawned` true)
      (`/Game/Blueprints/BillboardComponent.SetLookAtCamera` (`self.BillboardComponent`) true)
      (`KismetSystemLibrary.K2_SetTimerDelegate` (delegate `Attack_Event`) (`self.AttackSeconds`) true)
      ;[1 1 1] Test death
      (`KismetSystemLibrary.Delay` 4.0)
      (`KismetSystemLibrary.PrintString` "DIE")
      (`self.Die`))))

(event `Attack_Event`
  ;[1 1 1] After spawn animation finished
)

(event `self.ReceiveTick`
  (params (DeltaSeconds :type "Float (single-precision)"))
  (if (`self.IsSpawned`)
    (bind _shouldmove (`self.SetPlayerDirection`))
    (if _shouldmove
      (`self.MovePawn` DeltaSeconds))))

(fn `Damage`
  (params (Damage :type "Float (double-precision)"))
  (bind _output_get (set `self.CurrentHealth` (- (`self.CurrentHealth`) Damage)))
  (if (<= _output_get 0.0)
    (`self.Die`)))

(fn `DieTween`
  (params (T :type "Float (double-precision)"))
  (`/Game/Blueprints/BillboardComponent.GetBillboardActor` (`self.BillboardComponent`))
  (`self.K2_SetActorRelativeRotation` (`KismetMathLibrary.MakeRotator` (`KismetMathLibrary.Lerp` 0.0 90.0 T))))

(fn `Init`
  (params (Wave :type Integer) (PlayerPawn :type "Pawn Object Reference"))
  (set `self.CurrentWave` Wave)
  (set `self.PlayerPawn` PlayerPawn))

(fn `MovePawn`
  (params (DeltaTime :type "Float (double-precision)"))
  (`self.K2_SetActorLocation` (+ (* (`KismetMathLibrary.Normal` (`self.PlayerDirection`)) (`self.Speed`) DeltaTime) (`self.K2_GetActorLocation`))))

(fn `SetPlayerDirection`
  (returns (ShouldMove :type Boolean))
  (bind _playerpawn (`self.PlayerPawn`))
  (bind _minplayerdist (`self.MinPlayerDist`))
  (bind _returnvalue (- (`self.K2_GetActorLocation` _playerpawn) (`self.K2_GetActorLocation`)))
  (bind _returnvalue_2 (`KismetMathLibrary.VSizeSquared` _returnvalue))
  (bind _returnvalue_3 (>= _returnvalue_2 (* _minplayerdist _minplayerdist)))
  (`/Engine/EditorBlueprintResources/StandardMacros.IsValid` _playerpawn
    (:`Is Valid`
      (if _returnvalue_3
        (set `self.PlayerDirection` (/ _returnvalue (`KismetMathLibrary.Sqrt` _returnvalue_2))))
      (return _returnvalue_3))
    (:`Is Not Valid`
      (return false))))

(fn `SpawnTween`
  (params (T :type "Float (double-precision)"))
  (bind _newparam (`/Game/Blueprints/BillboardComponent.GetBillboardActor` (`self.BillboardComponent`)))
  (`self.K2_SetActorRelativeLocation` _newparam (`KismetMathLibrary.MakeVector` 0.0 0.0 (`KismetMathLibrary.Lerp` -100.0 0.0 T)) false true))

(fn `UserConstructionScript`)