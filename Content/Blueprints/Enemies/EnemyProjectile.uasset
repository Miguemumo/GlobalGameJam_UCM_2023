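; Enemy projectile actor that flies in a straight line and damages the player on overlap.
; Each Tick, Move applies a swept world offset from Direction, Speed and delta time until the Collided flag is set.
; Overlapping a Player calls its Damage function, spawns an ExplosionBillboard slightly offset along X, then destroys the projectile; other actors are ignored.
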(event `self.ReceiveActorBeginOverlap`
  (params (OtherActor :type "Actor Object Reference"))
  (bind (_returnvalue_location _returnvalue_rotation _returnvalue_scale) (`KismetMathLibrary.BreakTransform` (`self.GetTransform`)))
  (bind _asplayer (cast `/Game/Blueprints/Player/Player` OtherActor))
  (`/Game/Blueprints/Player/Player.Damage` _asplayer (`self.Damage`))
  (set `self.Collided` true)
  (`|SpawnActorFromClass` "/Game/Blueprints/ExplosionBillboard.ExplosionBillboard_C" (`KismetMathLibrary.MakeTransform` (+ _returnvalue_location (-50.0 0.0 0.0)) _returnvalue_rotation _returnvalue_scale) "AlwaysSpawn" "OverrideRootScale" null null)
  (`self.K2_DestroyActor`))

(event `self.ReceiveTick`
  (params (DeltaSeconds :type "Float (single-precision)"))
  (if (not (`self.Collided`))
    (`self.Move` DeltaSeconds)))

(fn `Move`
  (params (DeltaTime :type "Float (double-precision)"))
  (`self.K2_AddActorWorldOffset` (* DeltaTime (`self.Direction`) (`self.Speed`)) true))

(fn `UserConstructionScript`)