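; Player Blueprint that handles axis-driven movement and a basic health pool with a death callback.
; Tick runs DoMovement, which offsets the actor in world X and Y from the input axes, scaled by delta time and MovementSpeed.
; The Damage event lowers Health, clamped at zero, and calls OnDeath when it is depleted.
; AddHealth caps healing at MaxHealth, but the Heal event is empty and does not call it.
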(event `self.ReceiveTick`
  (params (DeltaSeconds :type "Float (single-precision)"))
  (`self.DoMovement` DeltaSeconds))

(event `Damage`
  (params (Damage :type "Float (double-precision)"))
  (`self.SubstracHealth` Damage))

(event `Heal`
  (params (Heal :type "Float (double-precision)")))

(fn `AddHealth`
  (params (NewParam :type "Float (double-precision)"))
  (set `self.Health` (`KismetMathLibrary.FMin` (+ (`self.Health`) NewParam) (`self.MaxHealth`))))

(fn `DoMovement`
  (params (DeltaTime :type "Float (double-precision)"))
  (bind _movementspeed (`self.MovementSpeed`))
  (`self.K2_AddActorWorldOffset` (`KismetMathLibrary.MakeVector` (* DeltaTime (`self.GetInputAxisValue`) 100.0 _movementspeed) (* DeltaTime (`self.GetInputAxisValue`) 100.0 _movementspeed))))

(fn `SubstracHealth`
  (params (Damage :type "Float (double-precision)"))
  (bind _output_get (set `self.Health` (`KismetMathLibrary.FMax` (- (`self.Health`) Damage))))
  (if (<= _output_get 0.0)
    (`self.OnDeath`)))

(fn `UserConstructionScript`)