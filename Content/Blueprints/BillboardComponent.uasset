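; An actor component that gives its owner a custom billboard.
; On BeginPlay it adds a ChildActorComponent to the owner, spawns a CustomBillboard through it, stores that actor and passes it the component's material instance.
; It exposes a getter for the billboard actor and SetLookAtCamera, which toggles the actor's AutoMove flag.
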(event `self.ReceiveBeginPlay`
  (bind _returnvalue (`|AddComponentByClass` :`self` (`self.GetOwner`) :`Class` "/Script/Engine.ChildActorComponent"))
  (`ChildActorComponent.SetChildActorClass` _returnvalue "/Game/Blueprints/CustomBillboard.CustomBillboard_C")
  (bind _ascustom_billboard (cast `/Game/Blueprints/CustomBillboard` (`ChildActorComponent.ChildActor` _returnvalue)))
  (bind _output_get (set `self.BillboardActor` _ascustom_billboard))
  (`/Game/Blueprints/CustomBillboard.Set Material Instance` _output_get (`self.MaterialInstance`)))

(fn `GetBillboardActor`
  (returns (NewParam :type "/Game/Blueprints/CustomBillboard Object Reference"))
  (return (`self.BillboardActor`)))

(fn `SetLookAtCamera`
  (params (bLook :type Boolean))
  (set `/Game/Blueprints/CustomBillboard.AutoMove` bLook (`self.BillboardActor`)))