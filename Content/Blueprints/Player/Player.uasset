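; Player Blueprint for a game with auto-attached weapons, leveling and stat upgrades, moved along two axes by a swept offset each tick.
; BeginPlay copies base stats, sets the camera view and spawns Scissors on the first of six grab points.
; Events forward to functions for damage, healing, regen, stat changes floored at base values, and weapon slots.
; Experience gains loop through level-up calls, recomputing a power-curve threshold, while zero health fires death or revive dispatchers.
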(event `self.ReceiveBeginPlay`
  (bind (_playerbasestats_weaponspeedincrease _playerbasestats_weaponsizeincrease _playerbasestats_weapondurationincrease _playerbasestats_weaponcooldown _playerbasestats_maxhealth _playerbasestats_pickuprange _playerbasestats_damage _playerbasestats_movementspeed _playerbasestats_revives _playerbasestats_expmultiplier) (break `/Game/Structs/PlayerStats` (`self.PlayerBaseStats`)))
  (`PlayerController.SetViewTargetWithBlend` (`GameplayStatics.GetPlayerController` 0) (`ActorComponent.GetOwner` (`self.Camera`)) 0.0 "VTBlend_Linear" 0.0 false)
  (set `self.PlayerStats` (make `/Game/Structs/PlayerStats` _playerbasestats_weaponspeedincrease _playerbasestats_weaponsizeincrease _playerbasestats_weapondurationincrease _playerbasestats_weaponcooldown _playerbasestats_maxhealth _playerbasestats_pickuprange _playerbasestats_damage _playerbasestats_movementspeed _playerbasestats_revives _playerbasestats_expmultiplier))
  (bind _returnvalue (`KismetSystemLibrary.K2_SetTimerDelegate` (delegate `Event Regen Health`)))
  (`KismetArrayLibrary.Array_Add` (`self.Timers`) _returnvalue)
  (set `self.WeaponSlots` (`|MakeArray` (`self.GrabPoint1`) (`self.GrabPoint2`) (`self.GrabPoint3`) (`self.GrabPoint4`) (`self.GrabPoint5`) (`self.GrabPoint6`)))
  (`self.AddWeapon` "/Game/Blueprints/Weapons/Scissors.Scissors_C"))

(event `self.ReceiveTick`
  (params (DeltaSeconds :type "Float (single-precision)"))
  (`self.Move` DeltaSeconds))

(event `Event Regen Health`
  (`self.RegenHealth`))

(event `Event Damage`
  (params (Amount :type "Float (double-precision)"))
  (`self.Damage` Amount))

(event `Event Heal`
  (params (Amount :type "Float (double-precision)"))
  (`self.Heal` Amount))

(event `Event Change Player Stats`
  (params (PlayerStatsChange :type "/Game/Structs/PlayerStats Structure (by ref)"))
  (`self.ChangePlayerStats` PlayerStatsChange))

(event `Event Gain Exp`
  (params (ExpAmount :type "Float (double-precision)"))
  (`self.ChangeEXP` ExpAmount))

(event `Event Add Weapon`
  (params (WeaponType :type "/Game/Blueprints/Weapons/WeaponBase Class Reference"))
  (`self.AddWeapon` WeaponType))

(fn `AddWeapon`
  (params (WeaponType :type "/Game/Blueprints/Weapons/WeaponBase Class Reference"))
  (bind _output (`|GetArrayItem` (`self.WeaponSlots`) (`self.NumWeapons`)))
  (if (< (`self.NumWeapons`) (`KismetArrayLibrary.Array_Length` (`self.WeaponSlots`)))
    (bind _returnvalue (`|SpawnActorFromClass` WeaponType (`self.GetTransform` (`ActorComponent.GetOwner` _output)) "Undefined" "OverrideRootScale" null null))
    (`/Engine/EditorBlueprintResources/StandardMacros.IncrementInt` (`self.NumWeapons`)
      (:`  `
        (`self.K2_AttachToComponent` _returnvalue _output "None" "KeepRelative" "KeepRelative" "KeepRelative" true)))))

(fn `CalculateNextExpCheckpoint`
  (set `self.ExpCheckPoint` (* (`self.BaseExp`) (`KismetMathLibrary.MultiplyMultiply_FloatFloat` (`KismetMathLibrary.Conv_IntToDouble` (`self.PlayerLevel`)) (`self.ExpFactorIncrease`)))))

(fn `ChangeEXP`
  (params (ExpAmount :type "Float (double-precision)"))
  (bind (_playerstats_weaponspeedincrease _playerstats_weaponsizeincrease _playerstats_weapondurationincrease _playerstats_weaponcooldown _playerstats_maxhealth _playerstats_pickuprange _playerstats_damage _playerstats_movementspeed _playerstats_revives _playerstats_expmultiplier) (break `/Game/Structs/PlayerStats` (`self.PlayerStats`)))
  (bind _output_get (set `self.CurrentExp` (+ (* ExpAmount _playerstats_expmultiplier) (`self.CurrentExp`))))
  (while (>= _output_get (`self.ExpCheckPoint`))
    (`self.OnLevelUp`)
    (set `self.CurrentExp` (- (`self.CurrentExp`) (`self.ExpCheckPoint`)))
    (`self.CalculateNextExpCheckpoint`)))

(fn `ChangePlayerStats`
  (params (`Player Stats Change` :type "/Game/Structs/PlayerStats Structure (by ref)"))
  (bind (_playerstats_weaponspeedincrease _playerstats_weaponsizeincrease _playerstats_weapondurationincrease _playerstats_weaponcooldown _playerstats_maxhealth _playerstats_pickuprange _playerstats_damage _playerstats_movementspeed _playerstats_revives) (break `/Game/Structs/PlayerStats` (`self.PlayerStats`)))
  (bind (_playerbasestats_weaponspeedincrease _playerbasestats_weaponsizeincrease _playerbasestats_weapondurationincrease _playerbasestats_weaponcooldown _playerbasestats_maxhealth _playerbasestats_pickuprange _playerbasestats_damage _playerbasestats_movementspeed _playerbasestats_revives) (break `/Game/Structs/PlayerStats` (`self.PlayerBaseStats`)))
  (set `self.PlayerStats` (make `/Game/Structs/PlayerStats` (`KismetMathLibrary.FMax` (+ `Player Stats Change_WeaponSpeedIncrease_4_DEFAB8A446A7319F5A50FFAB00A785E1` _playerstats_weaponspeedincrease) _playerbasestats_weaponspeedincrease) (`KismetMathLibrary.FMax` (+ `Player Stats Change_WeaponSizeIncrease_5_FA12BF1642D60BEAEF0434BD4D1A1703` _playerstats_weaponsizeincrease) _playerbasestats_weaponsizeincrease) (`KismetMathLibrary.FMax` (+ `Player Stats Change_WeaponDurationIncrease_7_689845454365F68F5A2715A89F0C1215` _playerstats_weapondurationincrease) _playerbasestats_weapondurationincrease) (`KismetMathLibrary.FMax` (+ `Player Stats Change_WeaponCooldown_9_B3503DF94C94E8D4CAF61A990274EBAF` _playerstats_weaponcooldown) _playerbasestats_weaponcooldown) (`KismetMathLibrary.FMax` (+ `Player Stats Change_MaxHealth_22_26ECA3CE4DD2243B273A2C83E8C77232` _playerstats_maxhealth) _playerbasestats_maxhealth) (`KismetMathLibrary.FMax` (+ `Player Stats Change_PickupRange_14_3AA4DBE04C99E7C2D84050ADBC687FF9` _playerstats_pickuprange) _playerbasestats_pickuprange) (`KismetMathLibrary.FMax` (+ `Player Stats Change_Damage_16_5C8E01AA46A9B62539299EA3970F1386` _playerstats_damage) _playerbasestats_damage) (`KismetMathLibrary.FMax` (+ 0.0 _playerstats_movementspeed) _playerbasestats_movementspeed) (`KismetMathLibrary.Max` (+ `Player Stats Change_Revives_21_5667D4DA46ED7E076D27EF8FE7177F20` _playerstats_revives) _playerbasestats_revives))))

(fn `Damage`
  (params (Damage :type "Float (double-precision)"))
  (bind (_playerstats_weaponspeedincrease _playerstats_weaponsizeincrease _playerstats_weapondurationincrease _playerstats_weaponcooldown _playerstats_maxhealth _playerstats_pickuprange _playerstats_damage _playerstats_movementspeed _playerstats_revives) (break `/Game/Structs/PlayerStats` (`self.PlayerStats`)))
  (bind _output_get (set `self.Health` (`KismetMathLibrary.FMax` (- (`self.Health`) Damage))))
  (if (<= _output_get 0.0)
    (if (> _playerstats_revives 0)
      (`self.OnDeath`)
      (for _array_element (`self.Timers`)
        (`KismetSystemLibrary.K2_ClearAndInvalidateTimerHandle` _array_element))
      (else
        (`self.OnRevive`)))))

(fn `Heal`
  (params (Heal :type "Float (double-precision)"))
  (bind (_playerstats_weaponspeedincrease _playerstats_weaponsizeincrease _playerstats_weapondurationincrease _playerstats_weaponcooldown _playerstats_maxhealth) (break `/Game/Structs/PlayerStats` (`self.PlayerStats`)))
  (set `self.Health` (`KismetMathLibrary.FMin` (+ (`self.Health`) Heal) _playerstats_maxhealth)))

(fn `Move`
  (params (DeltaTime :type "Float (double-precision)"))
  (bind (_playerstats_weaponspeedincrease _playerstats_weaponsizeincrease _playerstats_weapondurationincrease _playerstats_weaponcooldown _playerstats_maxhealth _playerstats_pickuprange _playerstats_damage _playerstats_movementspeed) (break `/Game/Structs/PlayerStats` (`self.PlayerStats`)))
  (`self.K2_AddActorWorldOffset` (`KismetMathLibrary.MakeVector` (* DeltaTime (`self.GetInputAxisValue`) 100.0 _playerstats_movementspeed) (* DeltaTime (`self.GetInputAxisValue`) 100.0 _playerstats_movementspeed)) true))

(fn `RegenHealth`
  (bind (_playerstats_weaponspeedincrease _playerstats_weaponsizeincrease _playerstats_weapondurationincrease _playerstats_weaponcooldown _playerstats_maxhealth) (break `/Game/Structs/PlayerStats` (`self.PlayerStats`)))
  (bind (_playerstats_weaponspeedincrease_2 _playerstats_weaponsizeincrease_2 _playerstats_weapondurationincrease_2 _playerstats_weaponcooldown_2 _playerstats_maxhealth_2 _playerstats_pickuprange _playerstats_damage _playerstats_movementspeed _playerstats_revives _playerstats_expmultiplier _playerstats_liferegen) (break `/Game/Structs/PlayerStats` (`self.PlayerStats`)))
  (bind (_playerstats_weaponspeedincrease_3 _playerstats_weaponsizeincrease_3 _playerstats_weapondurationincrease_3 _playerstats_weaponcooldown_3 _playerstats_maxhealth_3) (break `/Game/Structs/PlayerStats` (`self.PlayerStats`)))
  (if (< (`self.Health`) _playerstats_maxhealth)
    (set `self.Health` (`KismetMathLibrary.FMin` (+ (`self.Health`) _playerstats_liferegen) _playerstats_maxhealth_3))))

(fn `UserConstructionScript`)