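; CustomBillboard is an actor that shows a sprite plane which can turn to face the player camera.
; When AutoMove is set, Tick calls LookAtCamera, which sets SpritePivot's world rotation toward the first player's camera location using a look-at rotation.
; A separate SetMaterialInstance function swaps the first material slot on SpritePlane, allowing the displayed image to be changed.
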(event `self.ReceiveTick`
  (params (DeltaSeconds :type "Float (single-precision)"))
  (if (`self.AutoMove`)
    (`self.LookAtCamera`)))

(fn `LookAtCamera`
  (bind _spritepivot (`self.SpritePivot`))
  (`SceneComponent.K2_SetWorldRotation` _spritepivot (`KismetMathLibrary.FindLookAtRotation` (`SceneComponent.K2_GetComponentLocation` _spritepivot) (`PlayerCameraManager.GetCameraLocation` (`GameplayStatics.GetPlayerCameraManager` 0))) false false))

(fn `Set Material Instance`
  (params (MaterialInstance :type "MaterialInstance Object Reference"))
  (`PrimitiveComponent.SetMaterial` (`self.SpritePlane`) 0 MaterialInstance))

(fn `UserConstructionScript`)