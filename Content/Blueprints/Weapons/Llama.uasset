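; Llama weapon projectile that damages the first BaseEnemy it overlaps, spawns an ExplosionBillboard slightly above itself and destroys itself.
; Init supplies direction, speed and damage, and a BeginPlay delay destroys it when its lifetime ends.
; Tick sweeps it along that direction by a per-frame step not scaled by delta time, while rolling its Paper sprite at a time-scaled rate.
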(event `self.ReceiveBeginPlay`
  (`KismetSystemLibrary.Delay` (`self.Lifetime`))
  (`self.K2_DestroyActor`))

(event `Event Init`
  (params (Dir :type "Vector Structure") (Speed :type "Float (double-precision)") (Damage :type "Float (double-precision)"))
  (set `self.Dir` Dir)
  (set `self.Speed` Speed)
  (set `self.Damage` Damage))

(event `self.ReceiveTick`
  (params (DeltaSeconds :type "Float (single-precision)"))
  (bind _papersprite (`self.PaperSprite`))
  (`/Engine/EditorBlueprintResources/StandardMacros.IsValid` self
    (:`Is Valid`
      (`self.K2_AddActorWorldOffset` (* (`self.Dir`) (* (`self.Speed`) 100.0)) true)
      (`/Engine/EditorBlueprintResources/StandardMacros.IsValid` _papersprite
        (:`Is Valid`
          (`SceneComponent.K2_AddWorldRotation` _papersprite (`KismetMathLibrary.MakeRotator` (* DeltaSeconds 90.0)) false false))))))

(event `self.ReceiveActorBeginOverlap`
  (params (OtherActor :type "Actor Object Reference"))
  (bind (_returnvalue_x _returnvalue_y _returnvalue_z) (`KismetMathLibrary.BreakVector` (`self.K2_GetActorLocation`)))
  (bind _asbase_enemy (cast `/Game/Blueprints/Enemies/BaseEnemy` OtherActor))
  (`/Engine/EditorBlueprintResources/StandardMacros.IsValid` _asbase_enemy
    (:`Is Valid`
      (`/Game/Blueprints/Enemies/BaseEnemy.Damage` _asbase_enemy (`self.Damage`))
      (`|SpawnActorFromClass` "/Game/Blueprints/ExplosionBillboard.ExplosionBillboard_C" (`KismetMathLibrary.MakeTransform` (`KismetMathLibrary.MakeVector` _returnvalue_x _returnvalue_y (+ _returnvalue_z 10.0)) (struct) (1.5 1.5 1.5)) "Undefined" "OverrideRootScale" null null)
      (`self.K2_DestroyActor`))))

(fn `UserConstructionScript`)