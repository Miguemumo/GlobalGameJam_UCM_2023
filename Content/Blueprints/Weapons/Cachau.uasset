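; Cachau is a player weapon that deals area damage around the player on each shot, extending a parent weapon Blueprint.
; EventShoot calls DamageEnemies, triggers the player's EventTurnCachow, then plays the CachauGiro timeline to animate the Paper sprite's yaw.
; DamageEnemies runs a zero-length multi-sphere trace at the player's location and applies CurrentDamage to every BaseEnemy hit.
; LevelUp defers to the parent.
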(event `self.ReceiveBeginPlay`
  (`parent.ReceiveBeginPlay`))

(event `self.Event Shoot`
  (bind _papersprite (`self.PaperSprite`))
  (bind (_relativerotation_roll _relativerotation_pitch) (`KismetMathLibrary.BreakRotator` (`SceneComponent.RelativeRotation` _papersprite)))
  (`parent.Event Shoot`)
  (`self.DamageEnemies`)
  (`/Game/Blueprints/Player/Player.Event TurnCachow` (`self.PlayerRef`))
  (bind (_direction _cachaugiro) (`Timeline|CachauGiro` :!via `PlayFromStart`)
    (:`Update`
      (`SceneComponent.K2_SetRelativeRotation` _papersprite (`KismetMathLibrary.MakeRotator` _relativerotation_roll _relativerotation_pitch _cachaugiro) false false))))

(fn `DamageEnemies`
  (bind _returnvalue (`self.K2_GetActorLocation` (`self.PlayerRef`)))
  (bind (_outhits _returnvalue_2) (`KismetSystemLibrary.SphereTraceMulti` :`Start` _returnvalue :`End` _returnvalue :`Radius` (`self.Radius`) :`TraceChannel` "TraceTypeQuery3" :`DrawTime` 0.3))
  (if _returnvalue_2
    (for _array_element _outhits
      (bind _asbase_enemy (cast `/Game/Blueprints/Enemies/BaseEnemy` (`.HitActor` (`GameplayStatics.BreakHitResult` _array_element))))
      (`/Game/Blueprints/Enemies/BaseEnemy.Damage` _asbase_enemy (`self.CurrentDamage`)))))

(fn `LevelUp`
  (returns (CanLevelUp :type Boolean))
  (bind _canlevelup (`parent.LevelUp`))
  (return _canlevelup))

(fn `UserConstructionScript`
  (`parent.UserConstructionScript`))