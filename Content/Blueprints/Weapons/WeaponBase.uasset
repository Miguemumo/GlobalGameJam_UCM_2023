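; Base weapon Blueprint that handles cooldown-gated shooting and scales cooldown and damage by the owning player's stats.
; Init stores the player reference and runs RecalculateStats, which derives current values from base values and player multipliers.
; TryShoot counts the cooldown down by the supplied delta time and fires Shoot at zero or below.
; Shoot here only recalculates stats, resetting the cooldown; it contains no projectile or hit logic.
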(event `Event Try Shoot`
  (params (DeltaTime :type "Float (double-precision)"))
  (bind _shoot (`self.SubstactCooldown` DeltaTime))
  (if _shoot
    (`self.Event Shoot`)))

(event `Event Init`
  (params (PlayerRef :type "/Game/Blueprints/Player/Player Object Reference (by ref)"))
  (set `self.PlayerRef` PlayerRef)
  (`self.RecalculateStats` (`/Game/Blueprints/Player/Player.GetPlayerStats` (`self.PlayerRef`)) :!label _label))

(event `Event Shoot`
  (goto _label))

(fn `RecalculateStats`
  (params (PlayerStats :type "/Game/Structs/PlayerStats Structure (by ref)"))
  (set `self.CurrentCooldown` (- (* (`self.BaseCooldown`) PlayerStats_WeaponCooldown_9_B3503DF94C94E8D4CAF61A990274EBAF) (`self.CurrentCooldown`)))
  (set `self.CurrentDamage` (* (`self.BaseDamage`) PlayerStats_Damage_16_5C8E01AA46A9B62539299EA3970F1386)))

(fn `SubstactCooldown`
  (params (DeltaTime :type "Float (double-precision)"))
  (returns (Shoot :type Boolean))
  (bind _output_get (set `self.CurrentCooldown` (- (`self.CurrentCooldown`) DeltaTime)))
  (if (<= _output_get 0.0)
    (return true)
    (else
      (return false))))

(fn `UserConstructionScript`)