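; Cochinilla is a thrown explosive weapon projectile that damages enemies in an area when its lifetime expires.
; Init sets direction, speed and damage, then Tick sweeps it forward by a per-frame step not scaled by delta time and spins its Paper2D sprite.
; After the BeginPlay delay, a debug-drawn sphere trace damages BaseEnemy hits, then an explosion billboard spawns and the actor destroys itself.
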(event `self.ReceiveBeginPlay`
  (bind _returnvalue (`SceneComponent.K2_GetComponentLocation` (`self.Sphere`)))
  (`KismetSystemLibrary.Delay` (`self.Lifetime`))
  (bind (_outhits _returnvalue_2) (`KismetSystemLibrary.SphereTraceMulti` :`Start` _returnvalue :`End` _returnvalue :`Radius` 200.0 :`TraceChannel` "TraceTypeQuery3" :`DrawDebugType` "ForDuration" :`DrawTime` 2.0))
  (if _returnvalue_2
    (for _array_element _outhits
      (bind _asbase_enemy (cast `/Game/Blueprints/Enemies/BaseEnemy` (`.HitActor` (`GameplayStatics.BreakHitResult` _array_element))))
      (`/Game/Blueprints/Enemies/BaseEnemy.Damage` _asbase_enemy (`self.Damage`))))
  (`|SpawnActorFromClass` "/Game/Blueprints/ExplosionBillboard.ExplosionBillboard_C" (`KismetMathLibrary.MakeTransform` (`self.K2_GetActorLocation`) (struct) (2.0 2.0 2.0)) "AlwaysSpawn" "OverrideRootScale" null null)
  (`self.K2_DestroyActor`))

(event `Event Init`
  (params (Dir :type "Vector Structure") (Speed :type "Float (double-precision)") (Damage :type "Float (double-precision)"))
  (set `self.Dir` Dir)
  (set `self.Speed` Speed)
  (set `self.Damage` Damage))

(event `self.ReceiveTick`
  (params (DeltaSeconds :type "Float (single-precision)"))
  (`self.K2_AddActorWorldOffset` (* (`self.Dir`) (* (`self.Speed`) 100.0)) true)
  (`SceneComponent.K2_AddWorldRotation` (`self.PaperSprite`) (`KismetMathLibrary.MakeRotator` (* DeltaSeconds 180.0)) false false))

(fn `UserConstructionScript`)