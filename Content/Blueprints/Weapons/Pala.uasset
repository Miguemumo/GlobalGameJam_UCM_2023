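; Pala weapon that swings its root with a timeline and strikes beside the player on alternating sides.
; Each shot counts down CurrentAmount at 0.2-second intervals, spawning a player-attached PalaProyectile and damaging BaseEnemy actors through a separate multi box trace.
; RecalculateStats derives size and strike count from player stats.
; LevelUp raises base size and amount, swapping to the LastLevel visual at max level.
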(event `Event Level Up`
  (bind _level (`self.Level`))
  (if (< _level (`self.MaxLevel`))
    (bind _result (`/Engine/EditorBlueprintResources/StandardMacros.IncrementInt` _level)
      (:`  `
        (bind (_weaponspeedincrease _weaponsizeincrease _weapondurationincrease _weaponcooldown _maxhealth _pickuprange _damage) (break `/Game/Structs/PlayerStats` (`|GetArrayItem` (`self.LevelUpIncreases`) _result)))
        (set `self.BaseSize` (+ _weaponsizeincrease (`self.BaseSize`)))
        (set `self.BaseDamage` (+ _damage (`self.BaseDamage`)))))))

(event `self.ReceiveBeginPlay`
  (set `self.Rotation` (`SceneComponent.RelativeRotation` (`self.DefaultSceneRoot`))))

(event `self.Event Shoot`
  (bind (_rotation_roll _rotation_pitch _rotation_yaw) (`KismetMathLibrary.BreakRotator` (`self.Rotation`)))
  (bind _currentamount (`self.CurrentAmount`))
  (`parent.Event Shoot`)
  (`|ExecutionSequence`
    (:`then_0`
      (bind (_direction _newtrack_0) (`Timeline|Move` :!via `PlayFromStart`)
        (:`Update`
          (`SceneComponent.K2_SetRelativeRotation` (`self.DefaultSceneRoot`) (`KismetMathLibrary.MakeRotator` _rotation_roll _rotation_pitch (* _newtrack_0 (+ _rotation_yaw 30.0))) false false))))
    (:`then_1`
      (if (> _currentamount 0) :!label _label
        (`/Engine/EditorBlueprintResources/StandardMacros.DecrementInt` _currentamount
          (:`  `
            (`self.SpawnProjectile`)
            (`self.DamageEnemies`)
            (set `self.Side` (* (`self.Side`) -1))
            (`KismetSystemLibrary.Delay` 0.2)
            (goto _label)))
        (else
          (set `self.Side` 1))))))

(fn `DamageEnemies`
  (bind (_returnvalue_x _returnvalue_y _returnvalue_z) (`KismetMathLibrary.BreakVector` (/ (`KismetMathLibrary.Conv_DoubleToVector` (`self.CurrentSize`)) (2.0 2.0 2.0))))
  (bind _returnvalue (+ (`self.K2_GetActorLocation` (`self.PlayerRef`)) (`KismetMathLibrary.MakeVector` (* (+ _returnvalue_y (`self.Offset`)) (`self.Side`)) 0.0 _returnvalue_z)))
  (bind (_outhits _returnvalue_2) (`KismetSystemLibrary.BoxTraceMulti` :`Start` _returnvalue :`End` _returnvalue :`HalfSize` (`KismetMathLibrary.MakeVector` _returnvalue_x _returnvalue_y _returnvalue_z) :`TraceChannel` "TraceTypeQuery3" :`DrawTime` 0.2))
  (if _returnvalue_2
    (for _array_element _outhits
      (bind _asbase_enemy (cast `/Game/Blueprints/Enemies/BaseEnemy` (`.HitActor` (`GameplayStatics.BreakHitResult` _array_element))))
      (`/Game/Blueprints/Enemies/BaseEnemy.Damage` _asbase_enemy (`self.CurrentDamage`)))))

(fn `LevelUp`
  (returns (CanLevelUp :type Boolean))
  (bind (_weaponspeedincrease _weaponsizeincrease _weapondurationincrease _weaponcooldown _maxhealth _pickuprange _damage _movementspeed _revives _expmultiplier _liferegen _projectileamount) (break `/Game/Structs/PlayerStats` (`|GetArrayItem` (`self.LevelUpIncreases`) (`self.Level`))))
  (bind _canlevelup (`parent.LevelUp`))
  (if _canlevelup
    (set `self.BaseSize` (+ (`self.BaseSize`) _weaponsizeincrease))
    (set `self.BaseAmount` (+ (`self.CurrentAmount`) _projectileamount))
    (if (== (`self.Level`) (`self.MaxLevel`))
      (`SceneComponent.SetVisibility` (`self.PaperSprite`) false false)
      (`SceneComponent.SetVisibility` (`self.LastLevel`) true false)))
  (return _canlevelup))

(fn `RecalculateStats`
  (params (PlayerStats :type "/Game/Structs/PlayerStats Structure (by ref)"))
  (bind (_weaponspeedincrease _weaponsizeincrease _weapondurationincrease _weaponcooldown _maxhealth _pickuprange _damage _movementspeed _revives _expmultiplier _liferegen _projectileamount) (break `/Game/Structs/PlayerStats` PlayerStats))
  (`parent.RecalculateStats` PlayerStats)
  (set `self.CurrentSize` (* (`self.BaseSize`) _weaponsizeincrease))
  (set `self.CurrentAmount` (+ (`self.BaseAmount`) _projectileamount)))

(fn `SpawnProjectile`
  (bind (_returnvalue_x _returnvalue_y _returnvalue_z) (`KismetMathLibrary.BreakVector` (/ (`KismetMathLibrary.Conv_DoubleToVector` (`self.CurrentSize`)) (2.0 2.0 2.0))))
  (bind _returnvalue (`|SpawnActorFromClass` "/Game/Blueprints/Weapons/PalaProyectile.PalaProyectile_C" (`KismetMathLibrary.MakeTransform` (+ (`self.K2_GetActorLocation` (`self.PlayerRef`)) (`KismetMathLibrary.MakeVector` (* (+ _returnvalue_y (`self.Offset`)) (`self.Side`)) 0.0 _returnvalue_z)) (struct) (`KismetMathLibrary.Conv_DoubleToVector` (`self.BaseSize`))) "AlwaysSpawn" "OverrideRootScale" null null))
  (`/Game/Blueprints/Weapons/PalaProyectile.Event Init` _returnvalue (`self.Side`))
  (`self.K2_AttachToActor` _returnvalue (`self.PlayerRef`) "None" "KeepWorld" "KeepWorld" "KeepWorld" true))

(fn `UserConstructionScript`
  (`parent.UserConstructionScript`))