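; Herbicide puddle (charco) weapon actor that deals damage over time to enemies standing in it for a limited lifetime.
; Init scales the Sphere, sets the lifespan and damage rate, and nudges the actor slightly upward.
; Each Tick polls the Sphere for overlapping BaseEnemy actors and calls Damage on each, scaled by DeltaSeconds for a frame-rate-independent rate.
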(event `self.ReceiveTick`
  (params (DeltaSeconds :type "Float (single-precision)"))
  (for _array_element (`PrimitiveComponent.GetOverlappingActors` (`self.Sphere`) "/Game/Blueprints/Enemies/BaseEnemy.BaseEnemy_C")
    (bind _asbase_enemy (cast `/Game/Blueprints/Enemies/BaseEnemy` _array_element))
    (`/Game/Blueprints/Enemies/BaseEnemy.Damage` _asbase_enemy (* (`self.DamagePerSecond`) DeltaSeconds))))

(fn `Init`
  (params (Size :type "Float (double-precision)") (Duration :type "Float (double-precision)") (DamagePerSecond :type "Float (double-precision)"))
  (`SceneComponent.SetWorldScale3D` (`self.Sphere`) (`KismetMathLibrary.Conv_DoubleToVector` Size))
  (`self.SetLifeSpan` Duration)
  (set `self.DamagePerSecond` DamagePerSecond)
  (`self.K2_AddActorWorldOffset` (0.0 0.0 1.0) false true))

(fn `UserConstructionScript`)