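; Herbicide weapon that spawns a CharcoHerbicida puddle at the player's transform on each shot, initialized with current size, duration and damage per second.
; It extends a parent weapon class, adding per-level size and duration increases to the base values on level-up.
; Stat recalculation multiplies current size and duration by player modifiers.
; BeginPlay copies base size to current but assigns CurrentDuration to itself, not from BaseDuration.
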(event `self.ReceiveBeginPlay`
  (set `self.CurrentSize` (`self.BaseSize`))
  (set `self.CurrentDuration` (`self.CurrentDuration`)))

(event `self.Event Shoot`
  (bind _playerref (`self.PlayerRef`))
  (`parent.Event Shoot`)
  (bind _returnvalue (`|SpawnActorFromClass` "/Game/Blueprints/Weapons/CharcoHerbicida.CharcoHerbicida_C" (`self.GetTransform` _playerref) "AlwaysSpawn" "OverrideRootScale" null _playerref))
  (`/Game/Blueprints/Weapons/CharcoHerbicida.Init` _returnvalue (`self.CurrentSize`) (`self.CurrentDuration`) (`self.CurrentDamage`)))

(fn `LevelUp`
  (returns (CanLevelUp :type Boolean))
  (bind (_weaponspeedincrease _weaponsizeincrease _weapondurationincrease) (break `/Game/Structs/PlayerStats` (`|GetArrayItem` (`self.LevelUpIncreases`) (- (`self.Level`) 2))))
  (bind _canlevelup (`parent.LevelUp`))
  (set `self.BaseSize` (+ (`self.BaseSize`) _weaponsizeincrease))
  (set `self.BaseDuration` (+ (`self.BaseDuration`) _weapondurationincrease))
  (return _canlevelup))

(fn `RecalculateStats`
  (params (PlayerStats :type "/Game/Structs/PlayerStats Structure (by ref)"))
  (bind (_weaponspeedincrease _weaponsizeincrease _weapondurationincrease) (break `/Game/Structs/PlayerStats` PlayerStats))
  (`parent.RecalculateStats` PlayerStats)
  (set `self.CurrentSize` (* _weaponsizeincrease (`self.CurrentSize`)))
  (set `self.CurrentDuration` (* _weapondurationincrease (`self.CurrentDuration`)))
  (return))

(fn `UserConstructionScript`
  (`parent.UserConstructionScript`))