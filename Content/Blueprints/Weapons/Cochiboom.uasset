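; Cochiboom is a weapon Blueprint that fires a burst of Cochinilla projectiles from the player's location.
; On each shoot event it spawns the current amount of projectiles, initializing each with a direction from the Directions array, a fixed speed and the weapon's current damage.
; LevelUp runs the parent logic, then adds that level's projectile increase from LevelUpIncreases to the amount.
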(event `self.ReceiveBeginPlay`
  (set `self.player` (`GameplayStatics.GetPlayerPawn` 0)))

(event `self.Event Shoot`
  (`parent.Event Shoot`)
  (for _index (range (`self.CurrentAmount`))
    (bind _returnvalue (`|SpawnActorFromClass` "/Game/Blueprints/Weapons/Cochinilla.Cochinilla_C" (`KismetMathLibrary.MakeTransform` (`self.K2_GetActorLocation` (`GameplayStatics.GetPlayerPawn` 0))) "AlwaysSpawn" "OverrideRootScale" null null))
    (`/Game/Blueprints/Weapons/Cochinilla.Event Init` _returnvalue (`|GetArrayItem` (`self.Directions`) _index) 0.1 (`self.CurrentDamage`))))

(fn `LevelUp`
  (returns (CanLevelUp :type Boolean))
  (bind (_output_weaponspeedincrease _output_weaponsizeincrease _output_weapondurationincrease _output_weaponcooldown _output_maxhealth _output_pickuprange _output_damage _output_movementspeed _output_revives _output_expmultiplier _output_liferegen _output_projectileamount) (break `/Game/Structs/PlayerStats` (`|GetArrayItem` (`self.LevelUpIncreases`) (- (`self.Level`) 2))))
  (bind _canlevelup (`parent.LevelUp`))
  (set `self.CurrentAmount` (+ (`self.CurrentAmount`) _output_projectileamount))
  (return _canlevelup))

(fn `UserConstructionScript`
  (`parent.UserConstructionScript`))