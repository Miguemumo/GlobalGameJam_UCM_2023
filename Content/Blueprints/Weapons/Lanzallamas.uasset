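; Flamethrower weapon (Lanzallamas) that fires Llama flame projectiles from the player's location along four fixed diagonal directions on the XY plane.
; EventShoot extends the parent, spawning CurrentAmount sets of four in an undelayed loop, initializing each with speed and damage, then playing Anim.
; LevelUp raises base speed and amount from LevelUpIncreases when the parent call succeeds.
; RecalculateStats scales speed and adds to amount using PlayerStats.
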(event `self.Event Shoot`
  (`parent.Event Shoot`)
  (`|ExecutionSequence`
    (:`then_0`
      (for _ (range 1 (+ (`self.CurrentAmount`) 1))
        (bind _returnvalue (`|SpawnActorFromClass` "/Game/Blueprints/Weapons/Llama.Llama_C" (`KismetMathLibrary.MakeTransform` (`self.K2_GetActorLocation` (`self.PlayerRef`))) "Undefined" "OverrideRootScale" null null))
        (`/Engine/EditorBlueprintResources/StandardMacros.IsValid` _returnvalue
          (:`Is Valid`
            (`/Game/Blueprints/Weapons/Llama.Event Init` _returnvalue (0.707 0.707 0.0) (`self.CurrentSpeed`) (`self.CurrentDamage`))
            (bind _returnvalue_2 (`|SpawnActorFromClass` "/Game/Blueprints/Weapons/Llama.Llama_C" (`KismetMathLibrary.MakeTransform` (`self.K2_GetActorLocation` (`self.PlayerRef`))) "Undefined" "OverrideRootScale" null null))
            (`/Engine/EditorBlueprintResources/StandardMacros.IsValid` _returnvalue_2
              (:`Is Valid`
                (`/Game/Blueprints/Weapons/Llama.Event Init` _returnvalue_2 (0.707 -0.707 0.0) (`self.CurrentSpeed`) (`self.CurrentDamage`))
                (bind _returnvalue_3 (`|SpawnActorFromClass` "/Game/Blueprints/Weapons/Llama.Llama_C" (`KismetMathLibrary.MakeTransform` (`self.K2_GetActorLocation` (`self.PlayerRef`))) "Undefined" "OverrideRootScale" null null))
                (`/Engine/EditorBlueprintResources/StandardMacros.IsValid` _returnvalue_3
                  (:`Is Valid`
                    (`/Game/Blueprints/Weapons/Llama.Event Init` _returnvalue_3 (-0.707 0.707 0.0) (`self.CurrentSpeed`) (`self.CurrentDamage`))
                    (bind _returnvalue_4 (`|SpawnActorFromClass` "/Game/Blueprints/Weapons/Llama.Llama_C" (`KismetMathLibrary.MakeTransform` (`self.K2_GetActorLocation` (`self.PlayerRef`))) "Undefined" "OverrideRootScale" null null))
                    (`/Engine/EditorBlueprintResources/StandardMacros.IsValid` _returnvalue_4
                      (:`Is Valid`
                        (`/Game/Blueprints/Weapons/Llama.Event Init` _returnvalue_4 (-0.707 -0.707 0.0) (`self.CurrentSpeed`) (`self.CurrentDamage`))))))))))))
    (:`then_1`
      (`Timeline|Anim`))))

(fn `LevelUp`
  (returns (CanLevelUp :type Boolean))
  (bind (_weaponspeedincrease _weaponsizeincrease _weapondurationincrease _weaponcooldown _maxhealth _pickuprange _damage _movementspeed _revives _expmultiplier _liferegen _projectileamount) (break `/Game/Structs/PlayerStats` (`|GetArrayItem` (`self.LevelUpIncreases`) (- (`self.Level`) 2))))
  (bind _canlevelup (`parent.LevelUp`))
  (if _canlevelup
    (set `self.BaseSpeed` (+ (`self.BaseSpeed`) _weaponspeedincrease))
    (set `self.BaseAmount` (+ (`self.BaseAmount`) _projectileamount)))
  (return _canlevelup))

(fn `RecalculateStats`
  (params (PlayerStats :type "/Game/Structs/PlayerStats Structure (by ref)"))
  (bind (_weaponspeedincrease _weaponsizeincrease _weapondurationincrease _weaponcooldown _maxhealth _pickuprange _damage _movementspeed _revives _expmultiplier _liferegen _projectileamount) (break `/Game/Structs/PlayerStats` PlayerStats))
  (`parent.RecalculateStats` PlayerStats)
  (set `self.CurrentSpeed` (* (`self.BaseSpeed`) _weaponspeedincrease))
  (set `self.CurrentAmount` (+ (`self.BaseAmount`) _projectileamount))
  (return))

(fn `UserConstructionScript`
  (`parent.UserConstructionScript`))